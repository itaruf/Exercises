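; BP_LavaPool is a lava hazard actor that hurts the player character when it enters.
; On begin overlap it casts the other actor to ThirdPersonCharacter, subtracts DamageDealt from its Health and clamps the result to the character's MinHealth and MaxHealth.
; Health is changed directly, once per overlap with no damage over time, and the new value is printed for debugging.
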(event EventBeginPlay)

(event Collision|EventActorBeginOverlap
  (params (OtherActor :type Actor%20Object%20Reference))
  (bind _asthird_person_character (Utilities|Casting|CastToThirdPersonCharacter OtherActor))
  (bind _output_get (Variables|Default|SetAs%20Third%20Person%20Character _asthird_person_character))
  (bind _output_get_2 (Variables|/Game/ThirdPersonBP/Blueprints/ThirdPersonCharacter.ThirdPersonCharacter_C|SetHealth _output_get (Math|Float|Clamp(Float) (- (Variables|/Game/ThirdPersonBP/Blueprints/ThirdPersonCharacter.ThirdPersonCharacter_C|GetHealth (Variables|Default|GetAs%20Third%20Person%20Character)) (Variables|Default|GetDamageDealt)) (Variables|/Game/ThirdPersonBP/Blueprints/ThirdPersonCharacter.ThirdPersonCharacter_C|GetMinHealth (Variables|Default|GetAs%20Third%20Person%20Character)) (Variables|/Game/ThirdPersonBP/Blueprints/ThirdPersonCharacter.ThirdPersonCharacter_C|GetMaxHealth (Variables|Default|GetAs%20Third%20Person%20Character)))))
  (Development|PrintString (Utilities|String|ToString(Float) _output_get_2)))

(event EventTick
  (params (DeltaSeconds :type Float%20%28single-precision%29)))

(fn ConstructionScript)
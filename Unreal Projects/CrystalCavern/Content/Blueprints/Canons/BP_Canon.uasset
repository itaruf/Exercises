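; BP_Canon is a cannon that repeatedly fires on its own from BeginPlay, starting after a FireRate delay.
; A timeline animates the barrel's relative Y location, then spawns an actor on finish and restarts itself.
; Its Cannon Fired event track also loops back to the delay before replaying.
; The Projectile Properties graph supplies the spawn transform from ProjectileSpawnPoint and ProjectileScale.
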(event EventBeginPlay
  (bind (_returnvalue _returnvalue2 _projectilescale) (Utilities|ProjectileProperties))
  (Utilities|FlowControl|Delay (Variables|CanonProperties|GetFireRate) :!label _label)
  (bind _canon_barrel_location (Timeline|Canon%20Animation%20Timeline PlayFromStart)
    (:Update
      (Transformation|SetRelativeLocation (Variables|Default|GetCanonBarrel) (Math|Vector|MakeVector 0.0 _canon_barrel_location 0.0) false false))
    (:Finished
      (Game|SpawnActorfromClass "/Game/Blueprints/Projectiles/BP_Projectile.BP_Projectile_C" (Math|Transform|MakeTransform _returnvalue _returnvalue2 _projectilescale) "Undefined" 0 0)
      (Timeline|Canon%20Animation%20Timeline PlayFromStart))
    (:Cannon%20Fired
      (goto _label))))

(fn ConstructionScript)